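; BP_SkittlesZone is a trigger zone that plays a skittles sound when a BP_Bowl enters it.
; Its Box overlap filters for BP_Bowl, waits briefly, then passes a random index to PlayAudioSkittles, which sets that entry of Sounds on the Audio component and plays it.
; A branch picking the sound from the game manager's ScoreQuille is disconnected, so the GameManager reference cached at BeginPlay goes unused.
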(event OnComponentBeginOverlap(Box)
  (params (OverlappedComponent :type Primitive%20Component%20Object%20Reference) (OtherActor :type Actor%20Object%20Reference) (OtherComp :type Primitive%20Component%20Object%20Reference) (OtherBodyIndex :type Integer) (bFromSweep :type Boolean) (SweepResult :type Hit%20Result%20Structure%20%28by%20ref%29))
  (Utilities|Casting|CastToBP_Bowl OtherActor)
  (Utilities|FlowControl|Delay 0.4)
  (CallFunction|PlayAudioSkittles (Math|Random|RandomInteger 2)))

(event EventBeginPlay
  (bind _returnvalue (Actor|GetActorOfClass "/Game/MyContent/Assets/Blueprint/BP_GameManager.BP_GameManager_C"))
  (Variables|Default|SetgameManager _returnvalue))

(event Collision|EventActorBeginOverlap
  (params (OtherActor :type Actor%20Object%20Reference)))

(event EventTick
  (params (DeltaSeconds :type Float%20%28single-precision%29)))

(fn ConstructionScript)

(fn PlayAudioSkittles
  (params (soundIndex :type Integer))
  (Audio|Components|Audio|SetSound (Variables|Default|GetAudio) (Utilities|Array|Get(acopy) (Variables|Default|Getsounds) soundIndex))
  (Audio|Components|Audio|Play (Variables|Default|GetAudio) 0.0))